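; GC_CharacterBP is a player character Blueprint that carries a rifle and fires it on left mouse click.
; On BeginPlay it spawns a GC_Rifle_BP, stores it as CurrentWeapon and snaps it to the mesh's Weapon_Attach socket.
; It also adds a crosshair widget to the viewport.
; Pressing the left mouse button calls Fire on CurrentWeapon, leaving the firing logic to the weapon.
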(event `self.ReceiveBeginPlay`
  (bind _returnvalue (`|SpawnActorFromClass` "/Game/Blueprints/GC_Rifle_BP.GC_Rifle_BP_C" (`KismetMathLibrary.MakeTransform` (0.0 0.0 0.0)) "AlwaysSpawn" "OverrideRootScale" self null))
  (set `self.Current Weapon` _returnvalue)
  (`self.K2_AttachToComponent` _returnvalue (`self.Mesh`) "Weapon_Attach" "SnapToTarget" "SnapToTarget" "SnapToTarget" true)
  (bind _returnvalue_2 (`|CreateWidget` "/Game/UI/Crosshair_WGBP.Crosshair_WGBP_C"))
  (`UserWidget.AddToViewport` _returnvalue_2 0))

(event `Key|LeftMouseButton`
  (params (Key :type "Key Structure"))
  (:`Pressed`
    (`GC_WeaponBase.Fire` (`self.Current Weapon`))))

(fn `UserConstructionScript`)